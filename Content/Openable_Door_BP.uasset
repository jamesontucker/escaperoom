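; Openable door actor Blueprint that swings open and closed in response to OpenDoor's OnOpen and OnClose events.
; It stores its starting rotation on BeginPlay, then the DoorSwing timeline adds an animated yaw angle to that rotation, playing forward to open and reversing to close.
; An event track on the timeline plays a door lock sound at the actor's location.
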(event OnOpen(OpenDoor)
  ;[1 1 1] Set inital door rotation, On Open/Close door animate door's rotation
  (bind _open_angle (Timeline|Door%20Swing Play)
    (:Update
      (Transformation|SetActorRotation (Math|Rotator|CombineRotators (Variables|Default|GetInitialRotation) (Math|Rotator|MakeRotator 0.0 0.0 _open_angle))))
    (:Sound%20Timing
      (Audio|PlaySoundatLocation "/Game/Audio/door-lock.door-lock" (Transformation|GetActorLocation)))))

(event OnClose(OpenDoor)
  ;[1 1 1] Set inital door rotation, On Open/Close door animate door's rotation
  (bind _open_angle (Timeline|Door%20Swing Reverse)
    (:Update
      (Transformation|SetActorRotation (Math|Rotator|CombineRotators (Variables|Default|GetInitialRotation) (Math|Rotator|MakeRotator 0.0 0.0 _open_angle))))
    (:Sound%20Timing
      (Audio|PlaySoundatLocation "/Game/Audio/door-lock.door-lock" (Transformation|GetActorLocation)))))

(event EventBeginPlay
  ;[1 1 1] Set inital door rotation, On Open/Close door animate door's rotation
  (Variables|Default|SetInitialRotation (Transformation|GetActorRotation)))

(fn ConstructionScript)